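; Deer spawner actor that spawns a deer at BeginPlay and tries again whenever an actor tagged Player leaves its SpawnRange.
; Each valid spawn receives the spawner's Destinations list and has its die event bound back to the spawner.
; On that death it only calls ResetCanSpawn rather than spawning immediately, so a replacement waits for the player's next exit from range.
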(event `self.ReceiveBeginPlay`
  (bind _returnvalue (`self.Spawn` :!label _label))
  (`/Engine/EditorBlueprintResources/StandardMacros.IsValid` _returnvalue
    (:`Is Valid`
      (for _array_element (`self.destinations`)
        (`KismetArrayLibrary.Array_Add` (`EnemyBase.destinations_` _returnvalue) _array_element))
      (add `EnemyBase.dieEvent_` _returnvalue (delegate `die`)))))

(event `self.spawnRange.OnComponentEndOverlap`
  (params (OverlappedComponent :type "PrimitiveComponent Object Reference") (OtherActor :type "Actor Object Reference") (OtherComp :type "PrimitiveComponent Object Reference") (OtherBodyIndex :type Integer))
  (if (`self.ActorHasTag` OtherActor "Player")
    (goto _label)))

(event `die`
  (`self.ResetCanSpawn`))

(fn `UserConstructionScript`)