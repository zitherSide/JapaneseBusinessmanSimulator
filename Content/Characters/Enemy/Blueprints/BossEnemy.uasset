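; Boss enemy character whose fight begins when a player weapon hits its snap hitbox, blending the camera to it as the AI controller roars.
; ChargeAndFight adds the boss HUD and roars, then returns the camera and starts the AI fight.
; Kunai hits deal half damage, while body contact damages the player.
; Delegates make the skin glow during invincibility and stop AI before destroying it on death.
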(event `self.SnapHitBox.OnComponentBeginOverlap`
  (params (OverlappedComponent :type "PrimitiveComponent Object Reference") (OtherActor :type "Actor Object Reference") (OtherComp :type "PrimitiveComponent Object Reference") (OtherBodyIndex :type Integer) (bFromSweep :type Boolean) (SweepResult :type "HitResult Structure (by ref)"))
  ;[1 1 1] Snap
  (if (`self.ActorHasTag` OtherActor "playerWeapon")
    (set `PrimitiveComponent.bGenerateOverlapEvents` false (`self.SnapHitBox`))
    (`PlayerController.SetViewTargetWithBlend` (`GameplayStatics.GetPlayerController` 0) self 1.0 "VTBlend_Linear" 0.0 false)
    (bind _asboss_aicontroller (cast `/Game/Characters/Enemy/Behaviors/Boss/BossAIController` (`AIBlueprintHelperLibrary.GetAIController` self)))
    (`/Game/Characters/Enemy/Behaviors/Boss/BossAIController.Roar` _asboss_aicontroller)))

(event `RoarEvent`
  (bind _camerabacktime (`self.cameraBackTime`))
  ;[1 1 1] Start fight
  (`KismetSystemLibrary.Delay` (`self.chargeDurationSec_`))
  (`PlayerController.SetViewTargetWithBlend` (`GameplayStatics.GetPlayerController` 0) (`GameplayStatics.GetPlayerPawn` 0) _camerabacktime "VTBlend_Linear" 0.0 false)
  (`KismetSystemLibrary.Delay` _camerabacktime)
  (bind _asboss_aicontroller (cast `/Game/Characters/Enemy/Behaviors/Boss/BossAIController` (`AIBlueprintHelperLibrary.GetAIController` self)))
  (`/Game/Characters/Enemy/Behaviors/Boss/BossAIController.StartFight` _asboss_aicontroller))

(event `self.ReceiveBeginPlay`
  ;[1 1 1] Init
  (set `self.dieDelegate_` (delegate `カスタムイベント_2`))
  (bind _returnvalue (`PrimitiveComponent.CreateDynamicMaterialInstance` (`self.Mesh`) 3 "/Game/Characters/Enemy/Animation/Boss/Skin_MAT.Skin_MAT" "None"))
  (set `self.skinMaterial` _returnvalue)
  (set `self.startInvincibleDelegate_` (delegate `カスタムイベント_0`))
  (set `self.endInvincibleDelegate_` (delegate `カスタムイベント_1`))
  (bind _asboss_aicontroller (cast `/Game/Characters/Enemy/Behaviors/Boss/BossAIController` (`AIBlueprintHelperLibrary.GetAIController` self)))
  (`/Game/Characters/Enemy/Behaviors/Boss/BossAIController.StartTalk` _asboss_aicontroller)
  (set `PrimitiveComponent.bGenerateOverlapEvents` true (`self.SnapHitBox`)))

(event `カスタムイベント_0`
  ;[1 1 1] Init
  (`MaterialInstanceDynamic.SetScalarParameterValue` (`self.skinMaterial`) "Emission" 500.0))

(event `カスタムイベント_1`
  ;[1 1 1] Init
  (`MaterialInstanceDynamic.SetScalarParameterValue` (`self.skinMaterial`) "Emission" 0.0))

(event `カスタムイベント_2`
  ;[1 1 1] Dead
  (`BrainComponent.StopLogic` (`AIController.BrainComponent` (`AIBlueprintHelperLibrary.GetAIController` self)) "")
  (`KismetSystemLibrary.Delay` 2.0)
  (`self.K2_DestroyActor`))

(event `self.ReceiveTick`
  (params (DeltaSeconds :type "Float (single-precision)")))

(event `self.HitVolume.OnComponentBeginOverlap`
  (params (OverlappedComponent :type "PrimitiveComponent Object Reference") (OtherActor :type "Actor Object Reference") (OtherComp :type "PrimitiveComponent Object Reference") (OtherBodyIndex :type Integer) (bFromSweep :type Boolean) (SweepResult :type "HitResult Structure (by ref)"))
  (bind _askunai (cast `/Game/Characters/Player/Blueprints/KUnai` OtherActor :!pure true))
  ;[1 1 1] TakeDamage
  (if (`self.ActorHasTag` OtherActor "PlayerWeapon")
    (`GameplayStatics.ApplyDamage` self (/ (`ProjectileBase.damage_` _askunai) 2.0) null _askunai)
    (message `/Game/Characters/Player/Blueprints/IHitEffect.HitEffect` _askunai)))

(event `self.AttackVolume.OnComponentBeginOverlap`
  (params (OverlappedComponent :type "PrimitiveComponent Object Reference") (OtherActor :type "Actor Object Reference") (OtherComp :type "PrimitiveComponent Object Reference") (OtherBodyIndex :type Integer) (bFromSweep :type Boolean) (SweepResult :type "HitResult Structure (by ref)"))
  ;[1 1 1] Body Attack
  (bind _asjapanese_businessman_character (cast `JapaneseBusinessmanCharacter` OtherActor))
  (`GameplayStatics.ApplyDamage` _asjapanese_businessman_character (`self.bodyHitDamage_`)))

(fn `ChargeAndFight`
  (params (NewParam :type Boolean))
  (bind _returnvalue (`|CreateWidget` "/Game/UI/BossHUDBP.BossHUDBP_C"))
  (set `BossHUD.pawn_` self _returnvalue)
  (`UserWidget.AddToViewport` _returnvalue 0)
  (`self.InitialRoar`)
  (`AudioComponent.Play` (`self.Roar`) 0.0)
  (`self.RoarEvent`))

(fn `UserConstructionScript`)