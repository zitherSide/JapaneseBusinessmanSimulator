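; Base enemy Blueprint that handles contact damage to the player and damage taken from player projectiles.
; DamageBlock hits on Player-tagged actors apply the enemy's hit damage.
; HitVolume overlaps with PlayerWeapon-tagged actors, cast to ProjectileBase, apply the projectile's damage to the enemy, activate DamageParticle and destroy the projectile.
; BeginPlay binds DieAction, currently empty, to the die event.
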(event `self.ReceiveBeginPlay`
  (add `self.dieEvent_` (delegate `DieAction`)))

(event `DieAction`)

(event `self.DamageBlock.OnComponentHit`
  (params (HitComponent :type "PrimitiveComponent Object Reference") (OtherActor :type "Actor Object Reference") (OtherComp :type "PrimitiveComponent Object Reference") (NormalImpulse :type "Vector Structure") (Hit :type "HitResult Structure (by ref)"))
  ;[1 1 1] HitDamageToPlayer
  (if (`self.ActorHasTag` OtherActor "Player")
    (`GameplayStatics.ApplyDamage` OtherActor (`self.getHitDamage`) null self)))

(event `self.HitVolume.OnComponentBeginOverlap`
  (params (OverlappedComponent :type "PrimitiveComponent Object Reference") (OtherActor :type "Actor Object Reference") (OtherComp :type "PrimitiveComponent Object Reference") (OtherBodyIndex :type Integer) (bFromSweep :type Boolean) (SweepResult :type "HitResult Structure (by ref)"))
  (bind _asprojectile_base (cast `ProjectileBase` OtherActor :!pure true))
  ;[1 1 1] TakeDamge
  (if (`self.ActorHasTag` OtherActor "PlayerWeapon")
    (`GameplayStatics.ApplyDamage` self (`ProjectileBase.damage_` _asprojectile_base) null OtherActor)
    (`ActorComponent.Activate` (`self.DamageParticle`) true)
    (`self.K2_DestroyActor` _asprojectile_base)))

(fn `UserConstructionScript`)