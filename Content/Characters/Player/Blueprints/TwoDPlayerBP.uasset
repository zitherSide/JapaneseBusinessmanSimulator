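; Player character Blueprint for a 2D game, adding camera setup, a health HUD and a speed trail.
; BeginPlay applies the camera boom length and creates the PlayerHealthHUD widget with a reference to this pawn.
; Tick watches absolute Y velocity, starting TrailDummy once above a high threshold through a DoOnce, then stopping it and resetting the gate when speed drops.
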(event `self.ReceiveBeginPlay`
  (set `SpringArmComponent.TargetArmLength` (`self.cameraBoomLength`) (`self.CameraBoom`))
  (bind _returnvalue (`|CreateWidget` "/Game/UI/PlayerHealthHUD.PlayerHealthHUD_C" (`GameplayStatics.GetPlayerController` 0)))
  (set `PlayerHealthHUDBase.playerPawn_` self _returnvalue)
  (`UserWidget.AddToViewport` _returnvalue 0))

(event `self.ReceiveTick`
  (params (DeltaSeconds :type "Float (single-precision)"))
  (bind _traildummy (`self.TrailDummy`))
  (`|ExecutionSequence`
    (:`then_0`
      ;[1 1 1] C++からTrail表示をする場合終わる条件をどうするか？Dash||Jumpが終わったらかな？でもそれ判定するのTickになるよな...
      (if (> (`KismetMathLibrary.Abs` (.y (`MovementComponent.Velocity` (`self.GetMovementComponent`)))) 995.0)
        (`/Engine/EditorBlueprintResources/StandardMacros.DoOnce` false :!label _label
          (:`Completed`
            (`SkeletalMeshComponent.Play` _traildummy true)))
        (else
          (`SkeletalMeshComponent.Stop` _traildummy)
          (goto _label :!via `Reset`))))))

(fn `UserConstructionScript`)