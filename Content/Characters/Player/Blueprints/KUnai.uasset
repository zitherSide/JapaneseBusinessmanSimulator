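; KUnai is a kunai actor under the player Blueprints that handles its own spawn and hit feedback.
; It plays a spawn sound at its location on BeginPlay.
; Its HitEffect event plays a hit sound and activates the DamageParticle component; nothing in this graph calls that event.
; The overlap event is empty, and a disconnected branch that would destroy the actor unless the other actor is a JapaneseBusinessmanCharacter never runs.
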(event `self.ReceiveBeginPlay`
  (`GameplayStatics.PlaySoundAtLocation` (`self.SpawnSE`) (`self.K2_GetActorLocation`) (struct) 1.0 1.0 0.0 null null null))

(event `/Game/Characters/Player/Blueprints/IHitEffect.HitEffect`
  (`GameplayStatics.PlaySoundAtLocation` (`self.HitSE`) (`self.K2_GetActorLocation`) (struct) 1.0 1.0 0.0 null null null)
  (`ActorComponent.Activate` (`self.DamageParticle`) true))

(event `self.ReceiveActorBeginOverlap`
  (params (OtherActor :type "Actor Object Reference")))

(fn `UserConstructionScript`)