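; Base NPC character that shows a talk prompt when the player enters its region and runs a behavior-tree-driven conversation.
; BeginPlay passes its talk tree to TalkAIControllerBP, and Tick keeps the popup projected over the NPC.
; The popup's Next dispatcher freezes player movement, then plays an optional montage, blends to an optional talk camera and starts the AI talk.
; EndTalk restores the player camera and movement, stops the montage and removes the popup.
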(event `self.ReceiveBeginPlay`
  (`|ExecutionSequence`
    (:`then_0`
      (set `/Game/Characters/NPC/Behavior/TalkAIControllerBP.TalkTree` (`self.TalkBT`) (cast `/Game/Characters/NPC/Behavior/TalkAIControllerBP` (`AIBlueprintHelperLibrary.GetAIController` self) :!pure true)))))

(event `nextDispatcher__イベント_0`
  ;[1 1 1] Create PopupWidget
  (`Widget.RemoveFromParent` (`self.popUp_`))
  (`CharacterMovementComponent.DisableMovement` (`Character.CharacterMovement` (`GameplayStatics.GetPlayerCharacter` 0)))
  (`self.Talk`))

(event `self.popUpRegion_.OnComponentBeginOverlap`
  (params (OverlappedComponent :type "PrimitiveComponent Object Reference") (OtherActor :type "Actor Object Reference") (OtherComp :type "PrimitiveComponent Object Reference") (OtherBodyIndex :type Integer) (bFromSweep :type Boolean) (SweepResult :type "HitResult Structure (by ref)"))
  (bind _popup_ (`self.popUp_`))
  (if (`self.ActorHasTag` OtherActor "Player")
    (`|ExecutionSequence`
      (:`then_0`
        ;[1 1 1] Create PopupWidget
        (bind _returnvalue (`|CreateWidget` (`self.popUpType_`) (`GameplayStatics.GetPlayerController` 0)))
        (bind _output_get (set `self.popUp_` _returnvalue))
        (bind _asmessage_box_base (cast `MessageBoxBase` _output_get))
        (set `MessageBoxBase.content_` (`self.popUpContent_`) _asmessage_box_base)
        (add `MessageBoxBase.nextDispatcher_` _asmessage_box_base (delegate `nextDispatcher__イベント_0`)))
      (:`then_1`
        (`UserWidget.AddToViewport` _popup_ 0)
        (`UserWidget.SetPositionInViewport` _popup_ (`WidgetLayoutLibrary.ProjectWorldLocationToWidgetPosition` (`GameplayStatics.GetPlayerController` 0) (+ (`self.K2_GetActorLocation`) (`self.popUpPos_`))) false :!label _label)))))

(event `self.ReceiveTick`
  (params (DeltaSeconds :type "Float (single-precision)"))
  (`/Engine/EditorBlueprintResources/StandardMacros.IsValid` (`self.popUp_`)
    (:`Is Valid`
      (goto _label))))

(event `self.EndTalk`
  (`PlayerController.SetViewTargetWithBlend` (`GameplayStatics.GetPlayerController` 0) (`GameplayStatics.GetPlayerPawn` 0) 1.0 "VTBlend_Linear" 0.0 false)
  (`self.StopAnimMontage` (`self.talkingAnim_`))
  (`CharacterMovementComponent.SetMovementMode` (`Character.CharacterMovement` (`GameplayStatics.GetPlayerCharacter` 0)) "MOVE_Walking" 0)
  (`Widget.RemoveFromParent` (`self.popUp_`) :!label _label_2)
  (set `self.popUp_` null))

(event `self.popUpRegion_.OnComponentEndOverlap`
  (params (OverlappedComponent :type "PrimitiveComponent Object Reference") (OtherActor :type "Actor Object Reference") (OtherComp :type "PrimitiveComponent Object Reference") (OtherBodyIndex :type Integer))
  (`/Engine/EditorBlueprintResources/StandardMacros.IsValid` (`self.popUp_`)
    (:`Is Valid`
      (goto _label_2))))

(event `self.Talk`
  (bind _talkinganim_ (`self.talkingAnim_`))
  (`|ExecutionSequence`
    (:`then_0`
      (`/Engine/EditorBlueprintResources/StandardMacros.IsValid` _talkinganim_
        (:`Is Valid`
          (`self.PlayAnimMontage` _talkinganim_))))
    (:`then_1`
      (if (`self.usesTalkCamera`)
        (`PlayerController.SetViewTargetWithBlend` (`GameplayStatics.GetPlayerController` 0) self 1.0 "VTBlend_Linear" 0.0 false)))
    (:`then_2`
      (`/Game/Characters/NPC/Behavior/TalkAIControllerBP.Talk` (cast `/Game/Characters/NPC/Behavior/TalkAIControllerBP` (`AIBlueprintHelperLibrary.GetAIController` self) :!pure true)))))

(fn `ChangeCamera`)

(fn `StartAnim`)

(fn `UserConstructionScript`)