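; NPC character Blueprint for a guy in trouble who can take part in conversations.
; On BeginPlay it hands its TalkTree to its TalkAIControllerBP, provided that controller possesses it.
; The Talk event plays the talking montage, and EndTalk blends the first player controller's view target back to the player pawn.
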(event `self.ReceiveBeginPlay`
  (bind _astalk_aicontroller_bp (cast `/Game/Characters/NPC/Behavior/TalkAIControllerBP` (`self.GetController`)))
  (set `/Game/Characters/NPC/Behavior/TalkAIControllerBP.TalkTree` (`self.TalkTree`) _astalk_aicontroller_bp))

(event `/Game/Characters/NPC/Behavior/ITalkableBP.EndTalk`
  (`PlayerController.SetViewTargetWithBlend` (`GameplayStatics.GetPlayerController` 0) (`GameplayStatics.GetPlayerPawn` 0) 1.0 "VTBlend_Linear" 0.0 false))

(event `/Game/Characters/NPC/Behavior/ITalkableBP.Talk`
  (`self.PlayAnimMontage` (`self.talkingAnim_`)))

(fn `UserConstructionScript`)