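; Game mode Blueprint that runs a stage's lifecycle: BGM, game over, respawn, clear time and moving to the next level.
; GameOver counts deaths and, behind a DoOnce, plays the game-over song and message, halts the countdown and moves input from player to game mode.
; Pressing Talk or OK then respawns the player, restores music and input, restarts any timed countdown and resets the DoOnce.
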(event `self.ReceiveBeginPlay`
  (set `self.gameOverEvent_` (delegate `GameOver`)))

(event `GameOver`
  (bind _returnvalue (`GameplayStatics.GetPlayerController` 0))
  (`/Engine/EditorBlueprintResources/StandardMacros.IncrementInt` (`self.deathCount`)
    (:`  `
      (`/Engine/EditorBlueprintResources/StandardMacros.DoOnce` false :!label _label
        (:`Completed`
          (`self.PlayGameOver`)
          (`/Game/UI/InGameUI.ShowGameOverMessage` (cast `/Game/UI/InGameUI` (`self.currentWidget_`) :!pure true) true)
          (`self.DisableInput` (`self.player_`) _returnvalue)
          (`self.EnableInput` _returnvalue)
          (set `self.isGameOvering` true)
          (`self.StopCountdown`))))))

(event `self.ReceiveTick`
  (params (DeltaSeconds :type "Float (single-precision)")))

(event `InputAction|Talk`
  (params (Key :type "Key Structure"))
  (bind _returnvalue (`GameplayStatics.GetPlayerController` 0))
  (bind _asin_game_ui (cast `/Game/UI/InGameUI` (`self.currentWidget_`) :!pure true))
  (bind _startmessageshow (`/Game/UI/InGameUI.StartMessageShow` _asin_game_ui))
  (:`Pressed`
    (if (`self.isGameOvering`) :!label _label_2
      (`|ExecutionSequence`
        (:`then_0`
          (`self.DisableInput` _returnvalue)
          (`self.EnableInput` (`self.player_`) _returnvalue)
          (`self.RespawnPlayer`)
          (`/Game/UI/InGameUI.HideGameOverMessage` _asin_game_ui)
          (`UserWidget.PlayAnimation` _asin_game_ui _startmessageshow 0.0 1 "Forward" 1.0 false)
          (`UserWidget.PlayAnimation` _asin_game_ui _startmessageshow 0.0 1 "Reverse" 1.0 false)
          (`self.PlayBGM`))
        (:`then_1`
          (if (`self.hasTimeLimit_`)
            (`self.StartCountdown`)))
        (:`then_2`
          (set `self.isGameOvering` false))
        (:`then_3`
          (goto _label :!via `Reset`))))))

(event `InputAction|OK`
  (params (Key :type "Key Structure"))
  (:`Pressed`
    (goto _label_2)))

(fn `GetClearedTime`
  (returns (NewParam :type "Float (double-precision)"))
  (return (`self.consumedTime`)))

(fn `GetDeathCount`
  (returns (NewParam :type Integer))
  (return (`self.deathCount`)))

(fn `GotoNextStage`
  (`GameplayStatics.OpenLevel` (`self.nextLevel`))
  (set `self.deathCount` 0)
  (set `self.damageCount_` 0))

(fn `PlayBGM`
  (bind _currentbgm (`self.CurrentBGM`))
  (`AudioComponent.SetSound` _currentbgm (`self.stageSong`))
  (`AudioComponent.Play` _currentbgm 0.0))

(fn `PlayGameOver`
  (bind _currentbgm (`self.CurrentBGM`))
  (`AudioComponent.SetSound` _currentbgm (`self.gameOverSong`))
  (`AudioComponent.Play` _currentbgm 0.0))

(fn `StageClear`
  (set `self.consumedTime` (`GameplayStatics.GetTimeSeconds`))
  (`AudioComponent.SetSound` (`self.CurrentBGM`) (`self.clearSong`))
  (`AudioComponent.Play` (`self.CurrentBGM`) 0.0))

(fn `StageStart`
  (`self.PlayBGM`))

(fn `StartCountdown`
  (set `self.hasTimeLimit_` true)
  (set `self.currentTime_` (`self.timeLimit_`))
  (bind _returnvalue (`|CreateWidget` "/Game/UI/TimerWidget.TimerWidget_C" (`GameplayStatics.GetPlayerController` 0)))
  (bind _output_get (set `self.timerWidget_` _returnvalue))
  (`UserWidget.AddToViewport` _returnvalue 0)
  (`UserWidget.AddToViewport` _output_get 0)
  (set `self.isCountingDown_` true)
  (`UserWidget.PlayAnimation` _returnvalue (`/Game/UI/TimerWidget.StartTimer` _returnvalue) 0.0 1 "Forward" 1.0 false))

(fn `StopCountdown`
  (set `self.isCountingDown_` false))

(fn `UserConstructionScript`)